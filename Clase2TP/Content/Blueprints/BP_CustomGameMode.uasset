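; BP_CustomGameMode is a game mode that tracks a timed round and shows the score on screen.
; Each Tick adds delta time to CurrentTime, then prints Score, CurrentTime and MaxTime as debug text.
; Once the time limit is reached it prints a Spanish time-up message every frame; the QuitGame node is unconnected, so play continues.
; Score is only read here, never changed.
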(event EventBeginPlay)

(event EventTick
  (params (DeltaSeconds :type Float%20%28single-precision%29))
  ;[1 1 1] Print Score
  (Utilities|FlowControl|Sequence
    (:then_0
      (Variables|Default|SetcurrentTime (+ (Variables|Default|GetcurrentTime) DeltaSeconds)))
    (:then_1
      (Development|PrintString (Utilities|String|Append "Score: " (Utilities|String|ToString(Integer) (Variables|Default|GetScore)) "   " "Time: " (Utilities|String|ToString(Float) (Variables|Default|GetcurrentTime)) "/" (Utilities|String|ToString(Float) (Variables|Default|GetMaxTime))) true true "(R=0.000000,G=0.660000,B=1.000000,A=1.000000)" 0.0))
    (:then_2
      (if (>= (Variables|Default|GetcurrentTime) (Variables|Default|GetMaxTime))
        (Development|PrintString "SE ACABO EL TIEMPO")))))

(fn ConstructionScript)