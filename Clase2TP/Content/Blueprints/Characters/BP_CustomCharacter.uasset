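; BP_CustomCharacter is the player character for a Flappy Bird-style game, held motionless with zero gravity until the first input.
; A jump press or touch starts the game on first use, applying custom gravity and setting X velocity to Speed.
; Each press while falling launches the character upward by JumpForce, overriding vertical velocity.
; Tick and MoveRight do nothing; their movement logic is disconnected.
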(event EventBeginPlay
  ;[1 1 1] Comenzar con jugador en gravedad 0 y velocidad 0.
  (CallFunction|StopCharacterPlaying))

(event EventTick
  (params (DeltaSeconds :type Float%20%28single-precision%29))
  ;[1 0 0] No usados
)

(event Input|ActionEvents|InputActionJumpAction
  (params (Key :type Key%20Structure :default "None"))
  ;[1 1 1] Al apretar Input de Salto, empezar juego la primera vez, y llamar función LaunchCharacter cada vez.
  (:Pressed
    (if (Variables|Default|GetGameIsStarted?)
      _
      (else
        (CallFunction|StartGame)))
    (if (AI|Components|NavMovement|IsFalling (Variables|Character|GetCharacterMovement))
      (Character|LaunchCharacter (Math|Vector|MakeVector 0.0 0.0 (Variables|Default|GetJump%20Force)) false true))))

(event Input|AxisEvents|InputAxisMoveRight
  (params (AxisValue :type Float%20%28single-precision%29))
  ;[1 0 0] No usados
)

(event Input|TouchEvents|InputTouch
  (params (Location :type Vector) (FingerIndex :type ETouchIndex%20Enum))
  ;[1 1 1] Al apretar Input de Salto, empezar juego la primera vez, y llamar función LaunchCharacter cada vez.
  (:Pressed
    (if (Variables|Default|GetGameIsStarted?)
      _
      (else
        (CallFunction|StartGame)))
    (if (AI|Components|NavMovement|IsFalling (Variables|Character|GetCharacterMovement))
      (Character|LaunchCharacter (Math|Vector|MakeVector 0.0 0.0 (Variables|Default|GetJump%20Force)) false true))))

(fn ConstructionScript)

(fn StartGame
  ;[1 1 1] Comenzar a maxima velocidad (para mantener constante la velocidad en un juego tipo Flappy Bird)
  (Variables|Default|SetGameIsStarted? true)
  (bind _output_get (Variables|/Script/Engine.CharacterMovementComponent|SetMaxWalkSpeed (Variables|Character|GetCharacterMovement) (Variables|Default|GetSpeed)))
  (Variables|/Script/Engine.MovementComponent|SetVelocity (Variables|Character|GetCharacterMovement) (Math|Vector|MakeVector _output_get 0.0 0.0))
  (Variables|/Script/Engine.CharacterMovementComponent|SetGravityScale (Variables|Character|GetCharacterMovement) (Variables|Default|GetCustomGravity)))

(fn StopCharacterPlaying
  (bind _charactermovement (Variables|Character|GetCharacterMovement))
  (Variables|Default|SetGameIsStarted? false)
  (Variables|/Script/Engine.MovementComponent|SetVelocity _charactermovement "0, 0, 0")
  (Variables|/Script/Engine.CharacterMovementComponent|SetGravityScale _charactermovement 0.0))