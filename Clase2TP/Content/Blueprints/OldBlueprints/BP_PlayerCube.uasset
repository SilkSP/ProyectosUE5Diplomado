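; BP_PlayerCube is an early player cube that the player moves on the Y-Z plane through axis input.
; Movement offsets the actor location directly by axis value times Speed, without sweep or delta-time scaling.
; Collision overlaps drive gameplay through casts: the goal prints a win message, a moving hazard reloads Mapa1, and coins add their value to Score, print it and get destroyed.
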(event OnComponentBeginOverlap(Collision)
  (params (OverlappedComponent :type Primitive%20Component%20Object%20Reference) (OtherActor :type Actor%20Object%20Reference) (OtherComp :type Primitive%20Component%20Object%20Reference) (OtherBodyIndex :type Integer) (bFromSweep :type Boolean) (SweepResult :type Hit%20Result%20Structure%20%28by%20ref%29))
  (Utilities|Casting|CastToBP_Goal OtherActor
    (:then
      (Development|PrintString "GANASTE!"))
    (:CastFailed
      (Utilities|Casting|CastToBP_MovingHazard OtherActor
        (:then
          (Development|PrintString "DAÑOOOOO!!!!!")
          (Game|OpenLevel(byObjectReference) "/Game/Maps/Mapa1.Mapa1"))
        (:CastFailed
          (bind _asbp_coin (Utilities|Casting|CastToBP_Coin OtherActor))
          (Utilities|FlowControl|Sequence
            (:then_0
              (Variables|Default|SetScore (+ (Variables|Default|GetScore) (Variables|/Game/Blueprints/OldBlueprints/BP_Coin.BP_Coin_C|GetValue _asbp_coin))))
            (:then_1
              (Development|PrintString (Utilities|String|Append "Score: " (Utilities|String|ToString(Integer) (Variables|Default|GetScore)))))
            (:then_2
              (Actor|DestroyActor _asbp_coin))))))))

(event EventBeginPlay)

(event Collision|EventActorBeginOverlap
  (params (OtherActor :type Actor%20Object%20Reference)))

(event EventTick
  (params (DeltaSeconds :type Float%20%28single-precision%29)))

(event Input|AxisEvents|InputAxisMoveHorizontal
  (params (AxisValue :type Float%20%28single-precision%29))
  ;[1 1 1] Movimiento Horizontal
  (Transformation|SetActorLocation (+ (Transformation|GetActorLocation) (Math|Vector|MakeVector 0.0 (* AxisValue (Variables|Default|GetSpeed)) 0.0)) false false))

(event Input|AxisEvents|InputAxisMoveVertical
  (params (AxisValue :type Float%20%28single-precision%29))
  ;[1 1 1] Movimiento Vertical
  (Transformation|SetActorLocation (+ (Transformation|GetActorLocation) (Math|Vector|MakeVector 0.0 0.0 (* AxisValue (Variables|Default|GetSpeed)))) false false))

(fn ConstructionScript)