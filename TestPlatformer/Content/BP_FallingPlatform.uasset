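; BP_FallingPlatform is a platform that drops after a delay once the third-person character touches it.
; BeginPlay zeroes the ProjectileMovement gravity scale, and a Box overlap with BP_ThirdPersonCharacter sets IsFalling.
; While that flag is set, Tick accumulates time until MaxFallingTime, then restores gravity and clears the flag.
; The accumulated time is never reset, and leaving the box does not cancel the countdown.
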(event OnComponentBeginOverlap(Box)
  (params (OverlappedComponent :type Primitive%20Component%20Object%20Reference) (OtherActor :type Actor%20Object%20Reference) (OtherComp :type Primitive%20Component%20Object%20Reference) (OtherBodyIndex :type Integer) (bFromSweep :type Boolean) (SweepResult :type Hit%20Result%20Structure%20%28by%20ref%29))
  (Utilities|Casting|CastToBP_ThirdPersonCharacter OtherActor)
  (Variables|Default|SetisFalling true))

(event EventBeginPlay
  (Variables|/Script/Engine.ProjectileMovementComponent|SetProjectileGravityScale (Variables|Default|GetProjectileMovement) 0.0)
  (Variables|Default|SetisFalling false))

(event Collision|EventActorBeginOverlap
  (params (OtherActor :type Actor%20Object%20Reference)))

(event EventTick
  (params (DeltaSeconds :type Float%20%28single-precision%29))
  (if (Variables|Default|GetisFalling)
    (bind _output_get (Variables|Default|SetCurrentFallingTime (+ (Variables|Default|GetCurrentFallingTime) DeltaSeconds)))
    (if (>= _output_get (Variables|Default|GetMaxFallingTime))
      (Variables|/Script/Engine.ProjectileMovementComponent|SetProjectileGravityScale (Variables|Default|GetProjectileMovement) 1.0)
      (Variables|Default|SetisFalling false))))

(fn ConstructionScript)