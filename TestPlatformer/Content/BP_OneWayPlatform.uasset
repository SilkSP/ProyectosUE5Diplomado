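; One-way platform actor that lets the third-person character pass through its Cube mesh while airborne.
; Entering the DownCollision trigger while the character's movement reports falling disables the Cube's collision.
; Leaving the UpCollision trigger restores query and physics collision, regardless of movement state.
; Both triggers respond only to BP_ThirdPersonCharacter, and each toggle prints a debug message.
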(event OnComponentBeginOverlap(DownCollision)
  (params (OverlappedComponent :type Primitive%20Component%20Object%20Reference) (OtherActor :type Actor%20Object%20Reference) (OtherComp :type Primitive%20Component%20Object%20Reference) (OtherBodyIndex :type Integer) (bFromSweep :type Boolean) (SweepResult :type Hit%20Result%20Structure%20%28by%20ref%29))
  (bind _asbp_third_person_character (Utilities|Casting|CastToBP_ThirdPersonCharacter OtherActor))
  (if (AI|Components|NavMovement|IsFalling (Variables|/Script/Engine.Character|GetCharacterMovement _asbp_third_person_character))
    (Collision|SetCollisionEnabled (Variables|Default|GetCube) "NoCollision")
    (Development|PrintString (Utilities|String|Append (Utilities|GetDisplayName (Variables|Default|GetCube)) ": DISABLED"))))

(event OnComponentEndOverlap(UpCollision)
  (params (OverlappedComponent :type Primitive%20Component%20Object%20Reference) (OtherActor :type Actor%20Object%20Reference) (OtherComp :type Primitive%20Component%20Object%20Reference) (OtherBodyIndex :type Integer))
  (Utilities|Casting|CastToBP_ThirdPersonCharacter OtherActor)
  (Collision|SetCollisionEnabled (Variables|Default|GetCube) "QueryAndPhysics")
  (Development|PrintString (Utilities|String|Append (Utilities|GetDisplayName (Variables|Default|GetCube)) ": ENABLED")))

(event EventBeginPlay)

(event Collision|EventActorBeginOverlap
  (params (OtherActor :type Actor%20Object%20Reference)))

(event EventTick
  (params (DeltaSeconds :type Float%20%28single-precision%29)))

(fn ConstructionScript)